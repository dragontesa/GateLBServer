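; Game instance that holds the server match list and drives the matching server UI.
; It saves and loads the list through a BP_SaveGameServerMatch slot and exposes it as LBServerMatchInfo entries.
; Events create the W_MatchingServerUI widget, fill it from the list with auto-save suspended during the bulk add, and forward game ID and player count changes to it.
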(event `ShowServerMatchUI`
  (bind _returnvalue (`|CreateWidget` "/Game/UI/W_MatchingServerUI.W_MatchingServerUI_C"))
  (bind _output_get (set `self.W_ServerMatchUIRef` _returnvalue))
  (`UserWidget.AddToViewport` _output_get 0))

(event `SetupServerMatchUI`
  (bind _w_servermatchuiref (`self.W_ServerMatchUIRef`))
  (`/Engine/EditorBlueprintResources/StandardMacros.IsValid` _w_servermatchuiref
    (:`Is Valid`
      (set `/Game/UI/W_MatchingServerUI.IsAutoSave` false _w_servermatchuiref)
      (for _array_element (`self.ServerMatchMapDB`)
        (bind (_serverip _port) (break `/Game/Game/S_SaveGameServerMatch` _array_element))
        (`/Game/UI/W_MatchingServerUI.AddServerMatchEntry` (`self.W_ServerMatchUIRef`) (make `LBServerMatchInfo` 0 _port 0 0 _serverip)))
      (set `/Game/UI/W_MatchingServerUI.IsAutoSave` true (`self.W_ServerMatchUIRef`)))))

(event `UpdateServerMatchNewGameId`
  (params (ServerId :type Integer) (GameId :type Integer))
  (`/Game/UI/W_MatchingServerUI.UpdateServerMatchNewGameId` (`self.W_ServerMatchUIRef`) ServerId GameId))

(event `IncreaseGamePlayer`
  (params (ServerId :type Integer) (GameId :type Integer))
  (`/Game/UI/W_MatchingServerUI.IncreasePlayerNumbers` (`self.W_ServerMatchUIRef`) ServerId GameId))

(event `DecreaseGamePlayer`
  (params (ServerId :type Integer) (GameId :type Integer))
  (`/Game/UI/W_MatchingServerUI.DecreasePlayerNumbers` (`self.W_ServerMatchUIRef`) ServerId GameId))

(fn `GetGameServerMatchMap`
  (returns (OutMap :type "Array of LBServerMatchInfo Structure"))
  (locals (LBServerMatchMap :type "Array of LBServerMatchInfo Structure"))
  (for _array_element (`self.ServerMatchMapDB`)
    (bind (_serverip _port) (break `/Game/Game/S_SaveGameServerMatch` _array_element))
    (`KismetArrayLibrary.Array_Add` (`local.LBServerMatchMap`) (make `LBServerMatchInfo` 0 _port 0 0 _serverip)))
  (return (`local.LBServerMatchMap`)))

(fn `LoadGameServerMatch`
  (returns (GameServerMatchInfo :type "Array of /Game/Game/S_SaveGameServerMatch Structure"))
  (bind _servermatchmapdb (`self.ServerMatchMapDB`))
  (bind _returnvalue (`GameplayStatics.DoesSaveGameExist` "SaveGameServerMatchMap"))
  (if _returnvalue
    ;[0.02217 0.09759 0.3813] Load Server Match Info from saved File DB to Instance
    (bind _returnvalue_2 (`GameplayStatics.LoadGameFromSlot` "SaveGameServerMatchMap"))
    (bind _asbp_save_game_server_match (cast `/Game/Game/BP_SaveGameServerMatch` _returnvalue_2))
    (set `self.SaveGame_ServerMatchInfoMapRef` _asbp_save_game_server_match)
    (`KismetArrayLibrary.Array_Clear` _servermatchmapdb)
    (for _array_element (`/Game/Game/BP_SaveGameServerMatch.ServerMatchInfo` (`self.SaveGame_ServerMatchInfoMapRef`))
      (`KismetArrayLibrary.Array_Add` _servermatchmapdb _array_element))
    (else
      (`KismetSystemLibrary.PrintString` "Load game server match Failed !")))
  (return (`self.ServerMatchMapDB`)))

(fn `SaveGameServerMatch`
  (bind _savegame_servermatchinfomapref (`self.SaveGame_ServerMatchInfoMapRef`))
  (bind _servermatchinfo (`/Game/Game/BP_SaveGameServerMatch.ServerMatchInfo` _savegame_servermatchinfomapref))
  (`self.SaveGame_ServerMatchInfoMapRef`
    (:`then`
      _)
    (:`else`
      (bind _returnvalue (`GameplayStatics.CreateSaveGameObject` "/Game/Game/BP_SaveGameServerMatch.BP_SaveGameServerMatch_C"))
      (set `self.SaveGame_ServerMatchInfoMapRef` _returnvalue)))
  ;[0.02217 0.09759 0.3813] Update Server Match Map from Instance to SaveGame File DB
  (`KismetArrayLibrary.Array_Clear` _servermatchinfo)
  (for _array_element (`self.ServerMatchMapDB`)
    (`KismetArrayLibrary.Array_Add` _servermatchinfo _array_element))
  (`GameplayStatics.SaveGameToSlot` _savegame_servermatchinfomapref "SaveGameServerMatchMap"))