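; Game mode for the LB server that initializes the server and tracks game-server matches and their player counts.
; On BeginPlay it has the game instance load the match data and show its UI, then passes the match map to UpdateServerMatchMap.
; It binds to the LB server object's match-update and player increase/decrease events, forwarding each server and game ID to the game instance.
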(event `self.ReceiveBeginPlay`
  (`self.InitServer`)
  (bind _asbp_lbgame_instance (cast `/Game/Game/BP_LBGameInstance` (`GameplayStatics.GetGameInstance`))
    (:`then`
      (`/Game/Game/BP_LBGameInstance.LoadGameServerMatch` _asbp_lbgame_instance)
      (`/Game/Game/BP_LBGameInstance.ShowServerMatchUI` _asbp_lbgame_instance)
      (`/Game/Game/BP_LBGameInstance.SetupServerMatchUI` _asbp_lbgame_instance)
      (bind _outmap (`/Game/Game/BP_LBGameInstance.GetGameServerMatchMap` _asbp_lbgame_instance))
      (`self.UpdateServerMatchMap` _outmap)
      (bind _returnvalue (`self.GetLBServerObjectInstance`))
      (bind _output_get (set `self.LBServerObjRef` _returnvalue))
      (add `LBServerObject.UpdateGameServerMatchEvent` _output_get (delegate `OnUpdateGameServerMatch`))
      (add `LBServerObject.IncreaseGamePlayerEvent` _output_get (delegate `OnIncreaseGamePlayer`))
      (add `LBServerObject.DecreaseGamePlayerEvent` _output_get (delegate `DecreaseGamePlayer`)))
    (:`CastFailed`
      (`KismetSystemLibrary.PrintString` "Failure to get game instance"))))

(event `OnIncreaseGamePlayer`
  (params (id :type Integer) (GameId :type Integer))
  (`/Game/Game/BP_LBGameInstance.IncreaseGamePlayer` (stale `self.ReceiveBeginPlay` _asbp_lbgame_instance) id GameId))

(event `DecreaseGamePlayer`
  (params (id :type Integer) (GameId :type Integer))
  (`/Game/Game/BP_LBGameInstance.DecreaseGamePlayer` (stale `self.ReceiveBeginPlay` _asbp_lbgame_instance) id GameId))

(event `OnUpdateGameServerMatch`
  (params (id :type Integer) (GameId :type Integer))
  (`/Game/Game/BP_LBGameInstance.UpdateServerMatchNewGameId` (stale `self.ReceiveBeginPlay` _asbp_lbgame_instance) id GameId))

(fn `UserConstructionScript`)